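; BP_Test1 is a test actor that builds a straight row of instanced meshes and repeatedly prints a debug greeting during play.
; Its construction script randomly picks a floor, sphere or pillar mesh for one InstancedStaticMesh component, then adds evenly spaced instances using the actor's location and forward vector.
; BeginPlay starts an endless Delay loop that prints "Hello".
; An unconnected leftover applies the same random mesh pick to a Cube component.
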(event EventBeginPlay
  (Utilities|FlowControl|Delay 0.2 :!label _label)
  (Development|PrintString "Hello")
  (goto _label))

(event Collision|EventActorBeginOverlap
  (params (OtherActor :type Actor%20Object%20Reference)))

(event EventTick
  (params (DeltaSeconds :type Float%20%28single-precision%29)))

(fn ConstructionScript
  (bind _instancedstaticmesh (Variables|Default|GetInstancedStaticMesh))
  (Components|StaticMesh|SetStaticMesh _instancedstaticmesh (Utilities|Select :Index (Math|Random|RandomIntegerinRange 0 2) :Option%200 "/Game/StarterContent/Architecture/Floor_400x400.Floor_400x400" :Option%201 "/Engine/EditorMeshes/ArcadeEditorSphere.ArcadeEditorSphere" :Option%202 "/Game/StarterContent/Architecture/Pillar_50x500.Pillar_50x500"))
  (for _index (range 0 10)
    (Components|InstancedStaticMesh|AddInstance _instancedstaticmesh (Math|Transform|MakeTransform (+ (Transformation|GetActorLocation) (* (Transformation|GetActorForwardVector) 1e+02 _index)) "0, 0, 0" "1.000000,1.000000,1.000000") false)))