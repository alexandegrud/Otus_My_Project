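; BP_Door is a sliding double door that opens and closes through its OnOpen and OnClose events.
; BeginPlay caches each panel's starting relative location.
; The OpenClose timeline's DoorMove track drives a lerp that slides DoorL and DoorR in opposite directions by up to EndOffset from those starts, without sweep.
; OnOpen plays the timeline and OnClose reverses it.
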(event Custom|OnClose
  (bind _doormove (Timeline|OpenClose Reverse)
    (:Update
      (Transformation|SetRelativeLocation (Variables|Default|GetDoorL) (+ (Variables|Default|GetStartOffsetL) (* (Math|Vector|Lerp(Vector) "0, 0, 0" (- "" (Variables|Default|GetEndOffset)) _doormove) -1.0)) false false)
      (Transformation|SetRelativeLocation (Variables|Default|GetDoorR) (+ (Variables|Default|GetStartOffsetR) (Math|Vector|Lerp(Vector) "0, 0, 0" (- "" (Variables|Default|GetEndOffset)) _doormove)) false false))))

(event Custom|OnOpen
  (bind _doormove (Timeline|OpenClose Play)
    (:Update
      (Transformation|SetRelativeLocation (Variables|Default|GetDoorL) (+ (Variables|Default|GetStartOffsetL) (* (Math|Vector|Lerp(Vector) "0, 0, 0" (- "" (Variables|Default|GetEndOffset)) _doormove) -1.0)) false false)
      (Transformation|SetRelativeLocation (Variables|Default|GetDoorR) (+ (Variables|Default|GetStartOffsetR) (Math|Vector|Lerp(Vector) "0, 0, 0" (- "" (Variables|Default|GetEndOffset)) _doormove)) false false))))

(event EventBeginPlay
  (Variables|Default|SetStartOffsetR (Variables|/Script/Engine.SceneComponent|GetRelativeLocation (Variables|Default|GetDoorR)))
  (Variables|Default|SetStartOffsetL (Variables|/Script/Engine.SceneComponent|GetRelativeLocation (Variables|Default|GetDoorL))))

(fn ConstructionScript)