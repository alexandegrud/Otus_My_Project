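; BP_AIController_Boss is the AI controller for a boss, running the BT_AI_Boss behavior tree from BeginPlay.
; ActivateBoss creates a WB_BossHealth widget and adds it to the viewport, and DeactivateBoss removes it and clears the reference.
; While that widget is valid, Tick sets its health bar percent from Health divided by MaxHealth.
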(event Custom|Activate%20Boss
  (bind _returnvalue (UserInterface|CreateWidget "/Game/UI/WB_BossHealth.WB_BossHealth_C"))
  (bind _output_get (Variables|Default|SetBoss%20Health%20bat%20widget _returnvalue))
  (UserInterface|Viewport|AddtoViewport _output_get 0))

(event Custom|Deactivate%20Boss
  (Widget|RemovefromParent (Variables|Default|GetBoss%20Health%20bat%20widget))
  (Variables|Default|SetBoss%20Health%20bat%20widget 0))

(event EventBeginPlay
  (AI|RunBehaviorTree "/Game/AI/Boss/BT_AI_Boss.BT_AI_Boss"))

(event EventTick
  (params (DeltaSeconds :type Float%20%28single-precision%29))
  (bind _boss_health_bat_widget (Variables|Default|GetBoss%20Health%20bat%20widget)
    (:then
      (Progress|SetPercent (Variables|/Game/UI/WB_BossHealth.WB_BossHealth_C|GetHealthBar _boss_health_bat_widget) (/ (Variables|Default|GetHealth) (Variables|Default|GetMaxHealth))))
    (:else)))

(fn ConstructionScript
  (|CallParentFunction))