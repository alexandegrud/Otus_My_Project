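; BPC_Quest is a quest component that tracks the active quest's objectives and displays them on a quest HUD.
; It creates the WB_QuestHUD widget at BeginPlay, with events that push the quest name and objective list to it.
; EliminateEnemy removes the defeated enemy from each unfinished objective's elimination list, then marks emptied objectives completed and notifies the HUD.
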(event Custom|Set%20Active%20Quest%20Text
  (Rendering|Components|TextRender|SetText (Variables|/Game/Quest_System/WB_QuestHUD.WB_QuestHUD_C|GetActiveQuestText (Variables|Default|GetQuest%20Hud)) (Utilities|Text|ToText(String) (.Name (Utilities|Struct|BreakS_Quest (Variables|Default|GetactiveQuest))))))

(event Custom|Eliminate%20Enemy
  (params (Enemy%20Eliminated :type Actor%20Object%20Reference))
  (for _array_element (.objectives (Variables|Default|GetactiveQuest))
    (if (not (.Completed (Utilities|Struct|BreakS_Quest_Objective _array_element)))
      (if (> (Utilities|Array|Length (.ActorsToEliminate (Utilities|Struct|BreakS_Quest_Objective _array_element))) 0)
        (Utilities|Array|RemoveItem (.ActorsToEliminate (Utilities|Struct|BreakS_Quest_Objective _array_element)) Enemy%20Eliminated)
        (if (== (Utilities|Array|Length (.ActorsToEliminate (Utilities|Struct|BreakS_Quest_Objective _array_element))) 0)
          (|SetBy-RefVar _array_element (Utilities|Struct|MakeS_Quest_Objective (.NameAim (Utilities|Struct|BreakS_Quest_Objective _array_element)) true 0 0))
          (Default|CompleteObjective (Variables|Default|GetQuest%20Hud) _array_element))))))

(event Custom|Set%20Objectives
  (Default|FillObjectives (Variables|Default|GetQuest%20Hud) (.objectives (Variables|Default|GetactiveQuest))))

(event EventBeginPlay
  (bind _returnvalue (UserInterface|CreateWidget "/Game/Quest_System/WB_QuestHUD.WB_QuestHUD_C"))
  (bind _output_get (Variables|Default|SetQuest%20Hud _returnvalue))
  (UserInterface|Viewport|AddtoViewport _output_get 0))